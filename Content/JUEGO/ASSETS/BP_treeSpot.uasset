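; BP_treeSpot is a Christmas tree spot, apparently meant to award trees to the player, but its logic is currently inactive.
; ActivateNeighbor is an empty event, and the construction script is empty.
; One disconnected chain would reveal the tree, disable the Box's overlap events and play a bell sound.
; Another disconnected chain would show a "+N arbol" popup and add QTree to Life.
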(event EventActivateNeighbor
  (params (player :type VR%20Main%20Player%20Object%20Reference))
  ;[1 1 1] aumenta 1 arbol al jugador
)

(fn ConstructionScript)