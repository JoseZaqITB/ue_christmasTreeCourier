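; Enemy AI Blueprint that roams at random and chases the player character (PERSONAJE) when it sees it.
; Patrol starts on BeginPlay, moves to a random reachable point within a radius of its current location, and calls itself again on each successful move.
; PawnSensing sightings start a move toward the character and reset a short retriggerable delay, which resumes Patrol once sightings stop.
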(event OnSeePawn(PawnSensing)
  (params (Pawn :type Pawn%20Object%20Reference))
  ;[1 1 1] actuar solo si es Personaje
  (bind _aspersonaje (Utilities|Casting|CastToPERSONAJE Pawn))
  (Utilities|FlowControl|Sequence
    (:then_0
      ;[1 1 1] dirige el Pawn al target
      (AI|AIMoveTo self "0, 0, 0" _aspersonaje 5.0 false))
    (:then_1
      ;[1 1 1] cada que lo ve se ejecuta un delay que se resetea cada que lo ve, si deja de ver se espera 1s y vuelve a patrullar
      (Utilities|FlowControl|RetriggerableDelay 1.0)
      (CallFunction|Patrol))))

(event Custom|Patrol
  ;[1 1 1] genera movimiento aleatorio a un radio de 2500cm, siendo el origen el mismo
  (AI|AIMoveTo self (.RandomLocation (AI|Navigation|GetRandomReachablePointinRadius (Transformation|GetActorLocation) 2.5e+03 0 0)) 0 5.0 false
    (:OnSuccess
      ;[1 1 1] funcion que se llama asi misma
      (CallFunction|Patrol))))

(event EventBeginPlay
  (CallFunction|Patrol))

(fn ConstructionScript)